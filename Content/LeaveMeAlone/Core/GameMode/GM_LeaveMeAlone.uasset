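; Game mode for LeaveMeAlone that runs the level countdown and decides when a level is won or lost.
; A looping one-second timer decrements GameTime, shows Time Over at zero, and otherwise compares the CH_Player score with the level's threshold to show Next Level or Finish.
; An invalid player character records the death time, then triggers Game Over about two seconds later.
; Each end screen pauses the game and switches to UI-only input with a cursor.
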(event `self.ReceiveBeginPlay`
  (bind _returnvalue (`KismetSystemLibrary.K2_SetTimerDelegate` (delegate `CustomEvent`) 1.0 true))
  (set `self.GameTimerHandle` _returnvalue))

(event `CustomEvent`
  (bind _returnvalue (`GameplayStatics.GetPlayerCharacter` 0))
  (bind _output_get (set `self.GameTime` (- (`self.GameTime`) 1)))
  (if (== _output_get 0)
    (`KismetSystemLibrary.K2_ClearAndInvalidateTimerHandle` (`self.GameTimerHandle`))
    (bind _returnvalue_2 (`|CreateWidget` "/Game/LeaveMeAlone/Widgets/UI/WBP_TimeOver.WBP_TimeOver_C"))
    (`UserWidget.AddToViewport` _returnvalue_2 0)
    (`WidgetBlueprintLibrary.SetInputMode_UIOnlyEx` (`GameplayStatics.GetPlayerController` 0) null)
    (`GameplayStatics.SetGamePaused` true)
    (set `PlayerController.bShowMouseCursor` true (`GameplayStatics.GetPlayerController` 0))
    (else
      (`/Engine/EditorBlueprintResources/StandardMacros.IsValid` _returnvalue
        (:`Is Valid`
          (bind _asch_player (cast `/Game/LeaveMeAlone/Core/Character/CH_Player` _returnvalue))
          (bind _output_get_2 (set `self.ScoreFromPlayer` (`/Game/LeaveMeAlone/Core/Character/CH_Player.Score` _asch_player)))
          (if (== (`self.LevelNumber`) 1)
            (if (>= _output_get_2 (`self.ScoreForFirstLevel`))
              (bind _returnvalue_3 (`|CreateWidget` "/Game/LeaveMeAlone/Widgets/UI/WBP_NextLevel.WBP_NextLevel_C"))
              (`UserWidget.AddToViewport` _returnvalue_3 0)
              (`WidgetBlueprintLibrary.SetInputMode_UIOnlyEx` (`GameplayStatics.GetPlayerController` 0) null)
              (`GameplayStatics.SetGamePaused` true)
              (set `PlayerController.bShowMouseCursor` true (`GameplayStatics.GetPlayerController` 0)))
            (elif (>= _output_get_2 (`self.ScoreForSecondLevel`))
              (bind _returnvalue_4 (`|CreateWidget` "/Game/LeaveMeAlone/Widgets/UI/WBP_Finish.WBP_Finish_C"))
              (`UserWidget.AddToViewport` _returnvalue_4 0)
              (`WidgetBlueprintLibrary.SetInputMode_UIOnlyEx` (`GameplayStatics.GetPlayerController` 0) null)
              (`GameplayStatics.SetGamePaused` true)
              (set `PlayerController.bShowMouseCursor` true (`GameplayStatics.GetPlayerController` 0)))))
        (:`Is Not Valid`
          (if (== (`self.TimeDeath`) -1)
            (set `self.TimeDeath` (`self.GameTime`))
            (elif (>= (- (`self.TimeDeath`) (`self.GameTime`)) 2)
              (`KismetSystemLibrary.K2_ClearAndInvalidateTimerHandle` (`self.GameTimerHandle`))
              (bind _returnvalue_5 (`|CreateWidget` "/Game/LeaveMeAlone/Widgets/UI/WBP_GameOver.WBP_GameOver_C"))
              (`UserWidget.AddToViewport` _returnvalue_5 0)
              (`WidgetBlueprintLibrary.SetInputMode_UIOnlyEx` (`GameplayStatics.GetPlayerController` 0) null)
              (`GameplayStatics.SetGamePaused` true)
              (set `PlayerController.bShowMouseCursor` true (`GameplayStatics.GetPlayerController` 0)))))))))

(fn `UserConstructionScript`)